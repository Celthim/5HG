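; BP_MushroomWitch is a mushroom projectile in the boss GPE folder that damages the player and bursts into poison VFX.
; DoMovement snapshots its own and the player's locations, then a Timeline lerps between them with a height curve offset, so it does not home.
; Sphere overlap with the player applies damage.
; Impact or Timeline completion spawns the Niagara poison effect and destroys the actor.
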(event `PlayVFX`
  (`TimelineComponent.Stop` (`self.Movement`))
  (`NiagaraFunctionLibrary.SpawnSystemAtLocation` "/Game/VFX/FX/NiagaraSystems/NS_Poison.NS_Poison" (`self.K2_GetActorLocation`))
  (`/Engine/EditorBlueprintResources/StandardMacros.IsValid` self
    (:`Is Valid`
      (`self.K2_DestroyActor`))))

(event `self.ReceiveBeginPlay`
  (`KismetSystemLibrary.PrintString` "Hello"))

(event `DoMovement`
  (bind (_locationmushroom_x _locationmushroom_y _locationmushroom_z) (`KismetMathLibrary.BreakVector` (`self.LocationMushroom`)))
  (bind (_playerlocation_x _playerlocation_y _playerlocation_z) (`KismetMathLibrary.BreakVector` (`self.PlayerLocation`)))
  (set `self.LocationMushroom` (`self.K2_GetActorLocation`))
  (set `self.PlayerLocation` (`self.K2_GetActorLocation` (`/Game/Blueprints/Libraries/GlobalActorMacro_Lib.GetPlayer`)))
  (bind (_direction _alpha _location_z) (`Timeline|Movement` :!via `PlayFromStart`)
    (:`Update`
      (`self.K2_SetActorLocation` (`KismetMathLibrary.MakeVector` (`KismetMathLibrary.Lerp` _locationmushroom_x _playerlocation_x _alpha) (`KismetMathLibrary.Lerp` _locationmushroom_y _playerlocation_y _alpha) (`KismetMathLibrary.Lerp` _locationmushroom_z (+ _playerlocation_z _location_z) _alpha))))
    (:`Finished`
      (`/Engine/EditorBlueprintResources/StandardMacros.IsValid` self
        (:`Is Valid`
          (`self.PlayVFX`))))))

(event `self.Sphere.OnComponentBeginOverlap`
  (params (OverlappedComponent :type "PrimitiveComponent Object Reference") (OtherActor :type "Actor Object Reference") (OtherComp :type "PrimitiveComponent Object Reference") (OtherBodyIndex :type Integer) (bFromSweep :type Boolean) (SweepResult :type "HitResult Structure (by ref)"))
  (cast `/Game/Blueprints/Character/PlayerBP` OtherActor)
  (`/Game/Blueprints/Character/PC_Player.TakeDamage` (`/Game/Blueprints/Libraries/GlobalActorMacro_Lib.GetPC`) (`self.Damage`))
  (`self.PlayVFX`)
  (`/Engine/EditorBlueprintResources/StandardMacros.IsValid` self
    (:`Is Valid`
      (`self.K2_DestroyActor`))))

(fn `UserConstructionScript`)