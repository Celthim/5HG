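; Parent enemy Blueprint with health: it caches the player, makes a timed move on spawn, and destroys itself when damage depletes HP.
; A movement timeline lerps it toward a target XY with curve-driven height, and an event track triggers rotation.
; The mesh tumbles toward a random rotation, then a second timeline settles it on an axis-angle rotation computed from randomly picked arrow directions and the mesh's down vector.
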(event `Take Damage`
  (params (Damage :type "Float (double-precision)"))
  (bind _output_get (set `self.CurrentHp` (- (`self.CurrentHp`) Damage)))
  (if (<= _output_get 0.0)
    (set `self.IsDead` true)
    (`self.DetachFromControllerPendingDestroy`)
    (`/Engine/EditorBlueprintResources/StandardMacros.IsValid` self
      (:`Is Valid`
        (`self.K2_DestroyActor`)))))

(event `self.ReceiveAnyDamage`
  (params (Damage :type "Float (single-precision)") (DamageType :type "DamageType Object Reference") (InstigatedBy :type "Controller Object Reference") (DamageCauser :type "Actor Object Reference"))
  (`self.Take Damage` Damage))

(event `self.ReceiveBeginPlay`
  (`self.Init`))

(event `Init`
  (set `self.CurrentHp` (`self.MaxHp`))
  (set `self.RefPlayer` (cast `/Game/Blueprints/Character/PlayerBP` (`GameplayStatics.GetPlayerCharacter` 0) :!pure true))
  (`KismetArrayLibrary.Array_Append` (`self.Arrows`) (`|MakeArray` (`self.9`) (`self.10`) (`self.11`)))
  (`self.DoMovement`))

(event `DoMovement`
  (bind (_returnvalue_x _returnvalue_y _returnvalue_z) (`KismetMathLibrary.BreakVector` (`self.K2_GetActorLocation`)))
  (bind (_targetofdeplacement_x _targetofdeplacement_y) (`KismetMathLibrary.BreakVector` (`self.TargetOfDeplacement`)))
  (`TimelineComponent.SetPlayRate` (`self.TM_Deplacement`) (/ 1.0 (`self.TimeForMovement`)))
  (bind (_direction _alpha _z_location) (`Timeline|TM_Deplacement` :!via `PlayFromStart`)
    (:`Update`
      (`self.K2_SetActorLocation` (`KismetMathLibrary.MakeVector` (`KismetMathLibrary.Lerp` _returnvalue_x _targetofdeplacement_x _alpha) (`KismetMathLibrary.Lerp` _returnvalue_y _targetofdeplacement_y _alpha) (`KismetMathLibrary.Lerp` _returnvalue_z _z_location _alpha))))
    (:`BeginRotation`
      (`self.DoRotation`))))

(event `DoRotation`
  (bind _staticmesh (`self.StaticMesh`))
  (bind _staticmesh_2 (`self.StaticMesh`))
  (bind _arrows (`self.Arrows`))
  (bind _returnvalue (* (`SceneComponent.GetUpVector` (`self.StaticMesh`)) (0.0 0.0 -1.0)))
  (bind _returnvalue_2 (`SceneComponent.GetForwardVector` (`|GetArrayItem` _arrows (`KismetMathLibrary.RandomIntegerInRange` 0 (`KismetArrayLibrary.Array_LastIndex` _arrows)))))
  (`TimelineComponent.SetPlayRate` (`self.TM_Rotation`) (/ 1.0 (`self.TimeForRotation`)))
  (`SceneComponent.K2_SetWorldRotation` :`self` (`self.StaticMesh`))
  (set `self.TargetRot` (`KismetMathLibrary.RotatorFromAxisAndAngle` (`KismetMathLibrary.Normal` (`KismetMathLibrary.Cross_VectorVector` _returnvalue_2 _returnvalue)) (`KismetMathLibrary.DegAcos` (`KismetMathLibrary.Dot_VectorVector` _returnvalue_2 _returnvalue))))
  (set `self.RandomRotate` (`KismetMathLibrary.RandomRotator` true))
  (bind (_direction _alpha) (`Timeline|TM_Rotation` :!via `PlayFromStart`)
    (:`Update`
      (`SceneComponent.K2_SetRelativeRotation` _staticmesh (`KismetMathLibrary.RLerp` (`SceneComponent.RelativeRotation` _staticmesh) (`self.RandomRotate`) _alpha) false false))
    (:`Finished`
      (bind (_direction_2 _float) (`Timeline|TM_FinishRotate`)
        (:`Update`
          (`SceneComponent.K2_SetWorldRotation` _staticmesh_2 (`KismetMathLibrary.RLerp` (`SceneComponent.K2_GetComponentRotation` _staticmesh_2) (`self.TargetRot`) _float) false false))))))

(fn `UserConstructionScript`)