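; Base enemy Blueprint that handles health and a timeline-driven tumbling move, destroying itself when damage depletes its HP.
; On BeginPlay it moves toward a target location, with a timeline track shaping height.
; An event on that timeline starts a second timeline, spinning the mesh toward a random rotation.
; When the spin finishes, dot products pick the arrow pointing most downward, which drives a final actor rotation.
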(event `Take Damage`
  (params (Damage :type "Float (double-precision)"))
  (bind _output_get (set `self.CurrentHp` (- (`self.CurrentHp`) Damage)))
  (if (<= _output_get 0.0)
    (set `self.IsDead` true)
    (`self.DetachFromControllerPendingDestroy`)
    (`/Engine/EditorBlueprintResources/StandardMacros.IsValid` self
      (:`Is Valid`
        (`self.K2_DestroyActor`)))))

(event `self.ReceiveAnyDamage`
  (params (Damage :type "Float (single-precision)") (DamageType :type "DamageType Object Reference") (InstigatedBy :type "Controller Object Reference") (DamageCauser :type "Actor Object Reference"))
  (`self.Take Damage` Damage))

(event `self.ReceiveBeginPlay`
  (`self.Init`))

(event `Init`
  (set `self.CurrentHp` (`self.MaxHp`))
  (set `self.RefPlayer` (cast `/Game/Blueprints/Character/PlayerBP` (`GameplayStatics.GetPlayerCharacter` 0) :!pure true))
  (`self.DoMovement`))

(event `DoMovement`
  (bind (_returnvalue_x _returnvalue_y _returnvalue_z) (`KismetMathLibrary.BreakVector` (`self.K2_GetActorLocation`)))
  (bind (_targetofdeplacement_x _targetofdeplacement_y) (`KismetMathLibrary.BreakVector` (`self.TargetOfDeplacement`)))
  (`TimelineComponent.SetPlayRate` (`self.TM_Deplacement`) (/ 1.0 (`self.TimeForMovement`)))
  (bind (_direction _alpha _z_location) (`Timeline|TM_Deplacement` :!via `PlayFromStart`)
    (:`Update`
      (`self.K2_SetActorLocation` (`KismetMathLibrary.MakeVector` (`KismetMathLibrary.Lerp` _returnvalue_x _targetofdeplacement_x _alpha) (`KismetMathLibrary.Lerp` _returnvalue_y _targetofdeplacement_y _alpha) (`KismetMathLibrary.Lerp` _returnvalue_z _z_location _alpha))))
    (:`BeginRotation`
      (`self.DoRotation`))))

(event `DoRotation`
  (bind _staticmesh (`self.StaticMesh`))
  (`TimelineComponent.SetPlayRate` (`self.TM_Rotation`) (/ 1.0 (`self.TimeForRotation`)))
  (set `self.RandomRotate` (`KismetMathLibrary.RandomRotator` true))
  (bind (_direction _alpha) (`Timeline|TM_Rotation` :!via `PlayFromStart`)
    (:`Update`
      (`SceneComponent.K2_SetRelativeRotation` _staticmesh (`KismetMathLibrary.RLerp` (`SceneComponent.RelativeRotation` _staticmesh) (`self.RandomRotate`) _alpha) false false))
    (:`Finished`
      (for _array_element (`self.TabOfArrow`)
        (bind _returnvalue (`KismetMathLibrary.Dot_VectorVector` (`SceneComponent.GetForwardVector` _array_element) (* (`self.GetActorUpVector`) -1.0)))
        (if (> _returnvalue 0.0)
          (`/Engine/EditorBlueprintResources/StandardMacros.IsValid` (`self.GoodArrow`)
            (:`Is Valid`
              (if (< (`self.DotGoodArrow`) _returnvalue)
                (set `self.DotGoodArrow` _returnvalue)
                (set `self.GoodArrow` _array_element)))
            (:`Is Not Valid`
              (set `self.DotGoodArrow` _returnvalue)
              (set `self.GoodArrow` _array_element)))))
      (`self.K2_SetActorRotation` (`KismetMathLibrary.FindLookAtRotation` (`SceneComponent.GetForwardVector` (`self.GoodArrow`)) (* (`self.GetActorUpVector`) -1.0)))
      (set `self.GoodArrow` null)
      (set `self.DotGoodArrow` 0.0))))

(fn `UserConstructionScript`)