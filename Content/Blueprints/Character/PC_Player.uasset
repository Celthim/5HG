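; Player controller for a grid-based game where the player's mesh rolls like a die, cell by cell.
; Converts move input into camera-relative grid directions, then timelines tumble the mesh 90 degrees or arc it through bumper jumps with random spin.
; GridMovementCheck snaps to the Grid initially and refreshes allowed moves after each step; RefreshFaceUp finds the top face by dot product.
; Also handles camera, pause and damage, forwarding special-effect and reroll input to Celthim/Max interface actors.
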(event `Key|T`
  (params (Key :type "Key Structure"))
  (:`Pressed`
    (bind _outactors (`GameplayStatics.GetAllActorsOfClass` "/Game/Blueprints/Pawn/Enemy/BP_Enemy_Parent.BP_Enemy_Parent_C"))
    (for _array_element _outactors
      (`/Game/Blueprints/Pawn/Enemy/BP_Enemy_Parent.DoMovement` _array_element))))

(event `Unpause`
  ;[1 1 1] Pause
  (`/Game/Blueprints/Utilities/GameInstance/GI_Player.TogglePause` (`self.GI`) :!label _label))

(event `InputAxis|Turn Right / Left Mouse`
  (params (AxisValue :type "Float (single-precision)"))
  ;[0.05098 0.05098 0.05098] Camera Input - Mouse
  (`Pawn.AddControllerYawInput` (`self.Player BP`) AxisValue))

(event `InputAction|Pause` :paused true
  (params (Key :type "Key Structure"))
  ;[1 1 1] Pause
  (:`Released`
    (goto _label)))

(event `InputAction|Action Move Forward / Backward`
  (params (Key :type "Key Structure"))
  (bind _direction (`self.Direction`))
  (bind _returnvalue (or (== Key "Z") (== Key "W") (== Key "Gamepad_DPad_Up") (== Key "Gamepad_LeftStick_Up") (== Key "Up")))
  (bind (_returnvalue_x _returnvalue_y) (`KismetMathLibrary.BreakVector` (`SceneComponent.GetForwardVector` (`/Game/Blueprints/Character/PlayerBP.FollowCamera` (`/Game/Blueprints/Libraries/GlobalActorMacro_Lib.GetPlayer`)))))
  (bind _returnvalue_2 (not _returnvalue))
  (bind _returnvalue_3 (> _returnvalue_y 0.5))
  (bind _returnvalue_4 (< _returnvalue_y -0.5))
  (bind _returnvalue_5 (> _returnvalue_x 0.5))
  (bind _returnvalue_6 (< _returnvalue_x -0.5))
  ;[1 1 1] Event Movement
  (:`Pressed`
    (if (and (not (`self.InMovement`)) (not (`/Game/Blueprints/Libraries/GlobalActorMacro_Lib.IsFalling`)))
      (if (and _returnvalue _returnvalue_5)
        (set `self.Direction` "NewEnumerator0")
        (if (`self.isSpecialEffect`) :!label _label_2
          (`/Game/Blueprints/Character/PlayerInterfaceActor.Effect_Input` (`self.CelthimInterface`) _direction)
          (`/Game/Blueprints/Character/PlayerInterfaceActor.Effect_Input` (`self.MaxInterface`) _direction)
          (else
            (`self.DoMovement` _direction)))
        (elif (and _returnvalue_2 _returnvalue_5)
          (set `self.Direction` "NewEnumerator1")
          (goto _label_2)
          (elif (and _returnvalue_6 _returnvalue)
            (set `self.Direction` "NewEnumerator1")
            (goto _label_2)
            (elif (and _returnvalue_6 _returnvalue_2)
              (set `self.Direction` "NewEnumerator0")
              (goto _label_2)
              (elif (and _returnvalue_3 _returnvalue)
                (set `self.Direction` "NewEnumerator2")
                (goto _label_2)
                (elif (and _returnvalue_3 _returnvalue_2)
                  (set `self.Direction` "NewEnumerator3")
                  (goto _label_2)
                  (elif (and _returnvalue_4 _returnvalue)
                    (set `self.Direction` "NewEnumerator3")
                    (goto _label_2)
                    (elif (and _returnvalue_4 (not _returnvalue))
                      (set `self.Direction` "NewEnumerator2")
                      (goto _label_2))))))))))))

(event `self.ReceiveBeginPlay`
  ;[1 1 1] Init
  (`|ExecutionSequence`
    (:`then_0`
      (bind _output_get (set `self.CelthimInterface` (cast `/Game/Blueprints/Character/Celthim/PlayerInterfaceActor_Celthim` (`ChildActorComponent.ChildActor` (`self.PlayerInterfaceActor_Celthim`)) :!pure true)))
      (bind _output_get_2 (set `self.MaxInterface` (cast `/Game/Blueprints/Character/Max/PlayerInterfaceActor_Max` (`ChildActorComponent.ChildActor` (`self.PlayerInterfaceActor_Max`)) :!pure true)))
      (`/Game/Blueprints/Character/PlayerInterfaceActor.InitInterface` _output_get _output_get_2)
      (`/Game/Blueprints/Character/PlayerInterfaceActor.InitInterface` _output_get_2 _output_get)
      (bind _asplayer_bp (cast `/Game/Blueprints/Character/PlayerBP` (`GameplayStatics.GetPlayerCharacter` 0)))
      (set `self.Player BP` _asplayer_bp)
      (bind _asgi_player (cast `/Game/Blueprints/Utilities/GameInstance/GI_Player` (`GameplayStatics.GetGameInstance`)))
      (set `self.GI` _asgi_player))
    (:`then_1`
      (`UserWidget.AddToViewport` (`/Game/Blueprints/Utilities/GameInstance/GI_Player.PauseMenu` (`self.GI`)) 0)
      (set `self.CurrentHP` (`self.MaxHP`)))
    (:`then_2`
      (bind _returnvalue (`GameplayStatics.GetActorOfClass` "/Game/Blueprints/GPE/Grid/Grid.Grid_C"))
      (set `self.Grid` _returnvalue))
    (:`then_3`
      (`self.GridMovementCheck` false))))

(event `InputAxis|Look Up / Down Mouse`
  (params (AxisValue :type "Float (single-precision)"))
  ;[0.05098 0.05098 0.05098] Camera Input - Mouse
  (`Pawn.AddControllerPitchInput` (`self.Player BP`) AxisValue))

(event `InputAxis|Turn Right / Left Gamepad`
  (params (AxisValue :type "Float (single-precision)"))
  ;[0.05098 0.05098 0.05098] Camera Input - Gamepad
  (`Pawn.AddControllerYawInput` (`self.Player BP`) (* AxisValue (`self.BaseTurnRate`) (`GameplayStatics.GetWorldDeltaSeconds`))))

(event `TakeDamage`
  (params (Damage :type "Float (double-precision)"))
  (bind _output_get (set `self.CurrentHP` (- (`self.CurrentHP`) Damage)))
  (if (<= _output_get 0.0)
    (set `self.IsDead` true)))

(event `InputAxis|Look Up / Down Gamepad`
  (params (AxisValue :type "Float (single-precision)"))
  ;[0.05098 0.05098 0.05098] Camera Input - Gamepad
  (`Pawn.AddControllerPitchInput` (`self.Player BP`) (* AxisValue (`self.BaseLookUpRate`) (`GameplayStatics.GetWorldDeltaSeconds`))))

(event `self.ReceiveAnyDamage`
  (params (Damage :type "Float (single-precision)") (DamageType :type "DamageType Object Reference") (InstigatedBy :type "Controller Object Reference") (DamageCauser :type "Actor Object Reference"))
  (`self.TakeDamage` Damage))

(event `self.ReceiveTick`
  (params (DeltaSeconds :type "Float (single-precision)"))
  (`KismetSystemLibrary.PrintString` (`KismetStringLibrary.Conv_VectorToString` (`self.K2_GetActorLocation` (`/Game/Blueprints/Libraries/GlobalActorMacro_Lib.GetPlayer`))) true true (struct :`G` 0.66 :`B` 1.0 :`A` 1.0) 0.001)
  (`KismetSystemLibrary.PrintString` (`KismetStringLibrary.Conv_RotatorToString` (`SceneComponent.RelativeRotation` (`/Game/Blueprints/Character/PlayerBP.MeshPlayer` (`self.Player BP`)))) true true (struct :`R` 0.89 :`A` 1.0) 0.001))

(event `InputAction|Action Move Right / Left`
  (params (Key :type "Key Structure"))
  (bind _direction (`self.Direction`))
  (bind _returnvalue (or (== Key "Gamepad_DPad_Left") (== Key "Gamepad_LeftStick_Left") (== Key "Left") (== Key "Q") (== Key "A")))
  (bind (_returnvalue_x _returnvalue_y) (`KismetMathLibrary.BreakVector` (`SceneComponent.GetForwardVector` (`/Game/Blueprints/Character/PlayerBP.FollowCamera` (`/Game/Blueprints/Libraries/GlobalActorMacro_Lib.GetPlayer`)))))
  (bind _returnvalue_2 (not _returnvalue))
  (bind _returnvalue_3 (> _returnvalue_x 0.5))
  (bind _returnvalue_4 (< _returnvalue_x -0.5))
  (bind _returnvalue_5 (> _returnvalue_y 0.5))
  ;[1 1 1] Event Movement
  (:`Pressed`
    (if (and (not (`self.InMovement`)) (not (`/Game/Blueprints/Libraries/GlobalActorMacro_Lib.IsFalling`)))
      (if (and _returnvalue_3 _returnvalue)
        (set `self.Direction` "NewEnumerator3")
        (if (`self.isSpecialEffect`) :!label _label_3
          (`/Game/Blueprints/Character/PlayerInterfaceActor.Effect_Input` (`self.CelthimInterface`) _direction)
          (`/Game/Blueprints/Character/PlayerInterfaceActor.Effect_Input` (`self.MaxInterface`) _direction)
          (else
            (`KismetSystemLibrary.PrintString` (`|GetEnumeratorNameAsString` (`self.Direction`)))
            (`self.DoMovement` _direction)))
        (elif (and _returnvalue_3 _returnvalue_2)
          (set `self.Direction` "NewEnumerator2")
          (goto _label_3)
          (elif (and _returnvalue_4 _returnvalue)
            (set `self.Direction` "NewEnumerator2")
            (goto _label_3)
            (elif (and _returnvalue_4 _returnvalue_2)
              (set `self.Direction` "NewEnumerator3")
              (goto _label_3)
              (elif (and _returnvalue_5 _returnvalue)
                (set `self.Direction` "NewEnumerator0")
                (goto _label_3)
                (elif (and _returnvalue_5 _returnvalue_2)
                  (set `self.Direction` "NewEnumerator1")
                  (goto _label_3)
                  (elif (and (< _returnvalue_y -0.5) _returnvalue)
                    (set `self.Direction` "NewEnumerator1")
                    (goto _label_3)
                    (elif true
                      (set `self.Direction` "NewEnumerator0")
                      (goto _label_3))))))))))))

(event `DoMovement`
  (params (Direction :type "/Game/Blueprints/Utilities/Enum/Enum_Direction Enum" :default "NewEnumerator0"))
  (bind (_returnvalue _centerworldlocation) (`self.CheckMoveInput` Direction))
  (bind _relativerotationmeshplayer (`self.RelativeRotationMeshPlayer`))
  (bind _player_bp (`self.Player BP`))
  (bind (_actorlocationplayer_x _actorlocationplayer_y _actorlocationplayer_z) (`KismetMathLibrary.BreakVector` (`self.ActorLocationPlayer`)))
  (bind (_actorlocationplayer_x_2 _actorlocationplayer_y_2) (`KismetMathLibrary.BreakVector` (`self.ActorLocationPlayer`)))
  (bind (_actorlocationplayer_x_3 _actorlocationplayer_y_3) (`KismetMathLibrary.BreakVector` (`self.ActorLocationPlayer`)))
  (bind (_positiontarget_x _positiontarget_y) (`KismetMathLibrary.BreakVector` (`self.PositionTarget`)))
  (bind _player_bp_2 (`self.Player BP`))
  (bind _meshplayer (`/Game/Blueprints/Character/PlayerBP.MeshPlayer` (`self.Player BP`)))
  (`GameplayStatics.PlaySound2D` (select `int` (`KismetMathLibrary.RandomIntegerInRange` 0 2) :`0` "/Game/Sounds/FTPS_Gravel_01.FTPS_Gravel_01" :`1` "/Game/Sounds/FTPS_Gravel_02.FTPS_Gravel_02" :`2` "/Game/Sounds/FTPS_Gravel_03.FTPS_Gravel_03" :!type "SoundBase Object Reference") 1.0 1.0 0.0 null null)
  (if _returnvalue
    (set `self.PositionTarget` _centerworldlocation)
    (set `self.InMovement` true)
    (`TimelineComponent.SetPlayRate` (`self.TM_Movement`) (/ 1.0 (`self.TimeToMove`)))
    ;[1 1 1] Temp Variables
    (set `self.RelativeRotationMeshPlayer` (`SceneComponent.RelativeRotation` (`/Game/Blueprints/Character/PlayerBP.MeshPlayer` _player_bp_2)))
    (set `self.ActorLocationPlayer` (`self.K2_GetActorLocation` _player_bp_2))
    (bind (_direction _alpha _z_location) (`Timeline|TM_Movement` :!via `PlayFromStart`)
      (:`Update`
        (switch `/Game/Blueprints/Utilities/Enum/Enum_Direction` Direction
          (:`NewEnumerator0`
            ;[1 1 1] Set Rotation
            (`SceneComponent.K2_SetRelativeRotation` _meshplayer (`KismetMathLibrary.RLerp` _relativerotationmeshplayer (`KismetMathLibrary.ComposeRotators` _relativerotationmeshplayer (struct :`Roll` -90.0)) _alpha true) false false)
            (bind _returnvalue_2 (`KismetMathLibrary.Lerp` _actorlocationplayer_z (+ _actorlocationplayer_z _z_location) _alpha))
            ;[1 1 1] Set Location
            (`self.K2_SetActorLocation` _player_bp (`KismetMathLibrary.MakeVector` (`KismetMathLibrary.Lerp` _actorlocationplayer_x_3 _positiontarget_x _alpha) _actorlocationplayer_y_2 _returnvalue_2) false false))
          (:`NewEnumerator1`
            (`SceneComponent.K2_SetRelativeRotation` _meshplayer (`KismetMathLibrary.RLerp` _relativerotationmeshplayer (`KismetMathLibrary.ComposeRotators` _relativerotationmeshplayer (struct :`Roll` 90.0)) _alpha true) false false)
            (`self.K2_SetActorLocation` _player_bp (`KismetMathLibrary.MakeVector` (`KismetMathLibrary.Lerp` _actorlocationplayer_x_3 _positiontarget_x _alpha) _actorlocationplayer_y_2 _returnvalue_2) false false))
          (:`NewEnumerator2`
            (`SceneComponent.K2_SetRelativeRotation` _meshplayer (`KismetMathLibrary.RLerp` _relativerotationmeshplayer (`KismetMathLibrary.ComposeRotators` _relativerotationmeshplayer (struct :`Pitch` -90.0)) _alpha true) false false)
            (`self.K2_SetActorLocation` _player_bp (`KismetMathLibrary.MakeVector` _actorlocationplayer_x_2 (`KismetMathLibrary.Lerp` _actorlocationplayer_y_3 _positiontarget_y _alpha) _returnvalue_2) false false))
          (:`NewEnumerator3`
            (`SceneComponent.K2_SetRelativeRotation` _meshplayer (`KismetMathLibrary.RLerp` _relativerotationmeshplayer (`KismetMathLibrary.ComposeRotators` _relativerotationmeshplayer (struct :`Pitch` 90.0)) _alpha true) false false)
            (`self.K2_SetActorLocation` _player_bp (`KismetMathLibrary.MakeVector` _actorlocationplayer_x_2 (`KismetMathLibrary.Lerp` _actorlocationplayer_y_3 _positiontarget_y _alpha) _returnvalue_2) false false))))
      (:`Finished`
        (set `self.InMovement` false)
        (`self.GridMovementCheck` false)))))

(event `InputAction|SpecialEffect`
  (params (Key :type "Key Structure"))
  ;[1 1 1] SpecialEffect
  (:`Pressed`
    (if (not (`self.isSpecialEffect`))
      (`/Game/Blueprints/Character/PlayerInterfaceActor.UseSpecialEffect` (`self.CelthimInterface`) (`self.SpecialEffect`))
      (`/Game/Blueprints/Character/PlayerInterfaceActor.UseSpecialEffect` (`self.MaxInterface`) (`self.SpecialEffect`)))))

(event `SpecialEffectDilation`
  ;[1 1 1] SpecialEffect
  (`GameplayStatics.SetGlobalTimeDilation` 0.1)
  (`KismetSystemLibrary.Delay` 0.05)
  (`GameplayStatics.SetGlobalTimeDilation` 1.0))

(event `InputAction|Reroll`
  (params (Key :type "Key Structure"))
  ;[1 1 1] Reroll
  (:`Pressed`
    (if (not (`self.isSpecialEffect`))
      (`/Game/Blueprints/Character/PlayerInterfaceActor.UseReroll` (`self.CelthimInterface`) (`self.SpecialEffect`))
      (`/Game/Blueprints/Character/PlayerInterfaceActor.UseReroll` (`self.MaxInterface`) (`self.SpecialEffect`)))))

(event `Key|T`
  (params (Key :type "Key Structure"))
  (:`Pressed`
    (`/Game/Blueprints/Character/PlayerInterfaceActor.Test` (`self.CelthimInterface`))
    (`/Game/Blueprints/Character/PlayerInterfaceActor.Test` (`self.MaxInterface`))))

(event `DoJumpMovement`
  (params (Direction :type "/Game/Blueprints/Utilities/Enum/Enum_Direction Enum" :default "NewEnumerator0"))
  (bind _returnvalue (`KismetMathLibrary.RandomRotator` true))
  (bind (_returnvalue_2 _centerworldlocation) (`self.CheckMoveInput` Direction))
  (bind _tm_jumplocation (`self.TM_JumpLocation`))
  (bind (_positiontarget_x _positiontarget_y) (`KismetMathLibrary.BreakVector` (`self.PositionTarget`)))
  (bind _player_bp (`self.Player BP`))
  (bind _relativerotationmeshplayer (`self.RelativeRotationMeshPlayer`))
  (bind _player_bp_2 (`self.Player BP`))
  (bind (_actorlocationplayer_x _actorlocationplayer_y _actorlocationplayer_z) (`KismetMathLibrary.BreakVector` (`self.ActorLocationPlayer`)))
  (bind (_actorlocationplayer_x_2 _actorlocationplayer_y_2) (`KismetMathLibrary.BreakVector` (`self.ActorLocationPlayer`)))
  (bind (_actorlocationplayer_x_3 _actorlocationplayer_y_3) (`KismetMathLibrary.BreakVector` (`self.ActorLocationPlayer`)))
  (bind _meshplayer (`/Game/Blueprints/Character/PlayerBP.MeshPlayer` (`self.Player BP`)))
  (`GameplayStatics.PlaySound2D` "/Game/Sounds/Bumper.Bumper" 1.0 1.0 0.0 null null)
  (if _returnvalue_2
    (set `self.PositionTarget` _centerworldlocation)
    (set `self.InMovement` true)
    (`TimelineComponent.SetPlayRate` _tm_jumplocation (/ 1.0 (`self.TimeToMove`)))
    (`TimelineComponent.SetFloatCurve` _tm_jumplocation "/Game/Blueprints/Utilities/Curves/PlayerJumpZLocation.PlayerJumpZLocation" "Z Location")
    ;[1 1 1] Temp Variables
    (set `self.RelativeRotationMeshPlayer` (`SceneComponent.RelativeRotation` (`/Game/Blueprints/Character/PlayerBP.MeshPlayer` _player_bp)))
    (set `self.ActorLocationPlayer` (`self.K2_GetActorLocation` _player_bp))
    (bind (_direction _alpha _z_location _alphajump) (`Timeline|TM_JumpLocation` :!via `PlayFromStart`)
      (:`Update`
        (switch `/Game/Blueprints/Utilities/Enum/Enum_Direction` Direction
          (:`NewEnumerator0`
            ;[1 1 1] Set Rotation
            (`SceneComponent.K2_SetRelativeRotation` _meshplayer (`KismetMathLibrary.RLerp` _relativerotationmeshplayer (`KismetMathLibrary.ComposeRotators` _relativerotationmeshplayer _returnvalue) _alphajump true) false false)
            (set `self.FinishRotation` (`KismetMathLibrary.ComposeRotators` _relativerotationmeshplayer (struct :`Roll` -90.0)))
            (bind _returnvalue_3 (`KismetMathLibrary.Lerp` _actorlocationplayer_z (+ _actorlocationplayer_z _z_location) _alphajump))
            ;[1 1 1] Set Location
            (`self.K2_SetActorLocation` _player_bp_2 (`KismetMathLibrary.MakeVector` (`KismetMathLibrary.Lerp` _actorlocationplayer_x_3 _positiontarget_x _alpha) _actorlocationplayer_y_2 _returnvalue_3) false false))
          (:`NewEnumerator1`
            (`SceneComponent.K2_SetRelativeRotation` _meshplayer (`KismetMathLibrary.RLerp` _relativerotationmeshplayer (`KismetMathLibrary.ComposeRotators` _relativerotationmeshplayer _returnvalue) _alphajump true) false false)
            (set `self.FinishRotation` (`KismetMathLibrary.ComposeRotators` _relativerotationmeshplayer (struct :`Roll` 90.0)))
            (`self.K2_SetActorLocation` _player_bp_2 (`KismetMathLibrary.MakeVector` (`KismetMathLibrary.Lerp` _actorlocationplayer_x_3 _positiontarget_x _alpha) _actorlocationplayer_y_2 _returnvalue_3) false false))
          (:`NewEnumerator2`
            (`SceneComponent.K2_SetRelativeRotation` _meshplayer (`KismetMathLibrary.RLerp` _relativerotationmeshplayer (`KismetMathLibrary.ComposeRotators` _relativerotationmeshplayer _returnvalue) _alphajump true) false false)
            (set `self.FinishRotation` (`KismetMathLibrary.ComposeRotators` _relativerotationmeshplayer (struct :`Pitch` -90.0)))
            (`self.K2_SetActorLocation` _player_bp_2 (`KismetMathLibrary.MakeVector` _actorlocationplayer_x_2 (`KismetMathLibrary.Lerp` _actorlocationplayer_y_3 _positiontarget_y _alpha) _returnvalue_3) false false))
          (:`NewEnumerator3`
            (`SceneComponent.K2_SetRelativeRotation` _meshplayer (`KismetMathLibrary.RLerp` _relativerotationmeshplayer (`KismetMathLibrary.ComposeRotators` _relativerotationmeshplayer _returnvalue) _alphajump true) false false)
            (set `self.FinishRotation` (`KismetMathLibrary.ComposeRotators` _relativerotationmeshplayer (struct :`Pitch` 90.0)))
            (`self.K2_SetActorLocation` _player_bp_2 (`KismetMathLibrary.MakeVector` _actorlocationplayer_x_2 (`KismetMathLibrary.Lerp` _actorlocationplayer_y_3 _positiontarget_y _alpha) _returnvalue_3) false false))))
      (:`Finished`
        (`SceneComponent.K2_SetRelativeRotation` (`/Game/Blueprints/Character/PlayerBP.MeshPlayer` (`self.Player BP`)) (`self.FinishRotation`) false false)
        (set `self.InMovement` false)
        (`self.GridMovementCheck` false)))))

(fn `GridMovementCheck`
  (params (AllowOneZ :type Boolean))
  (bind _asplayer_bp (`/Game/Blueprints/Libraries/GlobalActorMacro_Lib.GetPlayer`))
  (bind _grid (`self.Grid`))
  (bind (_returnvalue_x _returnvalue_y _returnvalue_z) (`KismetMathLibrary.BreakVector` (`self.K2_GetActorLocation` (`/Game/Blueprints/Libraries/GlobalActorMacro_Lib.GetPlayer`))))
  (bind (_isongrid _x _y _centerworldlocation _z_index) (`/Game/Blueprints/GPE/Grid/Grid.Loc To Cell` _grid (`self.K2_GetActorLocation` _asplayer_bp)))
  (if _isongrid
    (`/Game/Blueprints/GPE/Grid/Grid.RefreshCanMove` _grid _x _y _z_index AllowOneZ)
    (set `self.X` _x)
    (set `self.Y` _y)
    (set `self.Z Index` _z_index)
    (if (not (`self.Init?`))
      (`self.K2_SetActorLocation` _asplayer_bp (`KismetMathLibrary.MakeVector` (.x _centerworldlocation) (.y _centerworldlocation) _returnvalue_z) false false)
      (set `self.Init?` true))))

(fn `Refresh Face Up`
  (locals (Index :type Integer :default 0) (dot :type "Float (double-precision)" :default -1.0))
  (for (_array_element _array_index) (`/Game/Blueprints/Character/PlayerBP.TabOfArrow` (`/Game/Blueprints/Libraries/GlobalActorMacro_Lib.GetPlayer`))
    (bind _returnvalue (`KismetMathLibrary.Dot_VectorVector` (`SceneComponent.GetForwardVector` _array_element) (`KismetMathLibrary.MakeVector` 0.0 0.0 1.0)))
    (if (> _returnvalue (`local.dot`))
      (set `local.dot` _returnvalue)
      (set `local.Index` _array_index)))
  (set `self.FaceUp` (+ (`local.Index`) 1)))

(fn `UserConstructionScript`)