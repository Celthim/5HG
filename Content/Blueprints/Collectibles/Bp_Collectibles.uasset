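; Collectible pickup with a configurable mesh, animated vertically by a timeline whose speed derives from a Time variable.
; On player overlap, it checks that both primary and secondary point totals on the player controller fall within set ranges.
; A valid pickup increments one total, optionally plays a volume-scaled sound and destroys itself.
; Secondary pickups also call Refresh on every BossParent actor to aggro bosses.
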(event `self.ReceiveBeginPlay`
  (bind _tm_movmenetup (`self.TM_MovmenetUp`))
  (`TimelineComponent.SetPlayRate` _tm_movmenetup (/ 1.0 (`self.Time`)))
  (`TimelineComponent.PlayFromStart` _tm_movmenetup))

(event `self.Box.OnComponentBeginOverlap`
  (params (OverlappedComponent :type "PrimitiveComponent Object Reference") (OtherActor :type "Actor Object Reference") (OtherComp :type "PrimitiveComponent Object Reference") (OtherBodyIndex :type Integer) (bFromSweep :type Boolean) (SweepResult :type "HitResult Structure (by ref)"))
  (bind _aspc_player (`/Game/Blueprints/Libraries/GlobalActorMacro_Lib.GetPC`))
  (bind _pointssecondary (`/Game/Blueprints/Character/PC_Player.PointsSecondary` (`/Game/Blueprints/Libraries/GlobalActorMacro_Lib.GetPC`)))
  (bind _pointsprimary (`/Game/Blueprints/Character/PC_Player.PointsPrimary` (`/Game/Blueprints/Libraries/GlobalActorMacro_Lib.GetPC`)))
  (cast `/Game/Blueprints/Character/PlayerBP` OtherActor)
  (if (and (>= _pointssecondary (`self.minSecondaryNeeded`)) (<= _pointssecondary (`self.maxSecondaryNeeded`)) (>= _pointsprimary (`self.minPrimaryNeeded`)) (<= _pointsprimary (`self.maxPrimaryNeeded`)))
    (if (not (`self.IsSecondary`))
      (`/Engine/EditorBlueprintResources/StandardMacros.IncrementInt` (`/Game/Blueprints/Character/PC_Player.PointsPrimary` _aspc_player)
        (:`  `
          _))
      (else
        (`/Engine/EditorBlueprintResources/StandardMacros.IncrementInt` (`/Game/Blueprints/Character/PC_Player.PointsSecondary` _aspc_player)
          (:`  `
            (`self.AggroBoss`)))))
    (if (`self.playSound`)
      (`GameplayStatics.PlaySoundAtLocation` "/Game/Sounds/Correct.Correct" (`self.K2_GetActorLocation`) (struct) (`.SFXVol` (`/Game/Blueprints/Libraries/GlobalActorMacro_Lib.getVol`)) 1.0 0.0 null null null null))
    (`/Engine/EditorBlueprintResources/StandardMacros.IsValid` self
      (:`Is Valid`
        (`self.K2_DestroyActor`)))))

(event `AggroBoss`
  (bind _outactors (`GameplayStatics.GetAllActorsOfClass` "/Game/Blueprints/GPE/Boss/BossParent.BossParent_C"))
  (for _array_element _outactors
    (`/Game/Blueprints/GPE/Boss/BossParent.Refresh` _array_element)))

(fn `UserConstructionScript`
  (`StaticMeshComponent.SetStaticMesh` (`self.StaticMesh`) (`self.Mesh`)))