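; Parent Blueprint for dice enemies, with empty events for actions, attacks, movement, damage and arrow setup.
; BeginPlay sets HP, caches the player and calls InitArrow.
; DoRotation tumbles the mesh randomly via timeline, then settles it on a rotation computed from randomly picked face arrows.
; Grid-based chasing, curve-driven hops per die type, timed action looping and damage/death logic remain in the graph but are disconnected, so never run.
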(event `Attack`)

(event `DoAction`)

(event `Take Damage`
  (params (Damage :type "Float (double-precision)")))

(event `self.ReceiveAnyDamage`
  (params (Damage :type "Float (single-precision)") (DamageType :type "DamageType Object Reference") (InstigatedBy :type "Controller Object Reference") (DamageCauser :type "Actor Object Reference")))

(event `self.ReceiveBeginPlay`
  (`self.Init`))

(event `Init`
  (set `self.CurrentHp` (`self.MaxHp`))
  (set `self.RefPlayer` (cast `/Game/Blueprints/Character/PlayerBP` (`GameplayStatics.GetPlayerCharacter` 0) :!pure true))
  (`self.InitArrow`))

(event `InitArrow`)

(event `DoMovement`)

(event `DoRotation`
  (bind _staticmesh (`self.StaticMesh`))
  (bind _staticmesh_2 (`self.StaticMesh`))
  (bind _arrows (`self.Arrows`))
  (bind _returnvalue (* (`SceneComponent.GetUpVector` (`self.StaticMesh`)) (0.0 0.0 -1.0)))
  (bind _returnvalue_2 (`SceneComponent.GetForwardVector` (`|GetArrayItem` _arrows (`KismetMathLibrary.RandomIntegerInRange` 0 (`KismetArrayLibrary.Array_LastIndex` _arrows)))))
  (`TimelineComponent.SetPlayRate` (`self.TM_Rotation`) (/ 1.0 (`self.TimeForRotation`)))
  (`SceneComponent.K2_SetWorldRotation` :`self` (`self.StaticMesh`))
  (set `self.TargetRot` (`KismetMathLibrary.RotatorFromAxisAndAngle` (`KismetMathLibrary.Normal` (`KismetMathLibrary.Cross_VectorVector` _returnvalue_2 _returnvalue)) (`KismetMathLibrary.DegAcos` (`KismetMathLibrary.Dot_VectorVector` _returnvalue_2 _returnvalue))))
  (set `self.RandomRotate` (`KismetMathLibrary.RandomRotator` true))
  (bind (_direction _alpha) (`Timeline|TM_Rotation` :!via `PlayFromStart`)
    (:`Update`
      (`SceneComponent.K2_SetRelativeRotation` _staticmesh (`KismetMathLibrary.RLerp` (`SceneComponent.RelativeRotation` _staticmesh) (`self.RandomRotate`) _alpha) false false))
    (:`Finished`
      (bind (_direction_2 _float) (`Timeline|TM_FinishRotate`)
        (:`Update`
          (`SceneComponent.K2_SetWorldRotation` _staticmesh_2 (`KismetMathLibrary.RLerp` (`SceneComponent.K2_GetComponentRotation` _staticmesh_2) (`self.TargetRot`) _float) false false))
        (:`Finished`
          (`SceneComponent.K2_SetWorldRotation` _staticmesh_2 (`self.TargetRot`) false false))))))

(fn `Chope la loc de la Grid`
  (params (CenterWorldLocation :type "Vector Structure"))
  (returns (`LaBonneLocation ;)` :type "Vector Structure"))
  (bind (_x _y) (`KismetMathLibrary.BreakVector3f` CenterWorldLocation))
  (bind _outhit (`KismetSystemLibrary.LineTraceSingleByProfile` CenterWorldLocation (+ CenterWorldLocation (0.0 0.0 -500.0))))
  (return (`KismetMathLibrary.MakeVector` _x _y (.z (`.ImpactPoint` (`GameplayStatics.BreakHitResult` _outhit))))))

(fn `UserConstructionScript`)