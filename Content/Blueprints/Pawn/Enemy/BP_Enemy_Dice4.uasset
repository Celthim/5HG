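; Enemy pawn Blueprint, apparently the Dice4 variant of a parent enemy class that supplies the actual behavior.
; Its InitArrow event appends a fixed four-entry sequence to the Arrows array, setting this variant's arrow pattern.
; BeginPlay and the construction script only call their parent versions.
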(event `self.ReceiveBeginPlay`
  (`parent.ReceiveBeginPlay`))

(event `self.InitArrow`
  (`KismetArrayLibrary.Array_Append` (`self.Arrows`) (`|MakeArray` (`self.1`) (`self.2`) (`self.4`) (`self.3`))))

(fn `UserConstructionScript`
  (`parent.UserConstructionScript`))