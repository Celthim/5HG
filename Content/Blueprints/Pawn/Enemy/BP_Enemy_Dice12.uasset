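; Enemy pawn Blueprint for the Dice12 enemy variant, apparently a twelve-sided die.
; It overrides the InitArrow event to append a fixed, shuffled order of the numbers 1 to 12 to the Arrows array.
; BeginPlay is disabled and the construction script only calls the parent, so this file adds no other logic.
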(event `self.InitArrow`
  (`KismetArrayLibrary.Array_Append` (`self.Arrows`) (`|MakeArray` (`self.2`) (`self.12`) (`self.10`) (`self.9`) (`self.6`) (`self.5`) (`self.1`) (`self.4`) (`self.3`) (`self.11`) (`self.7`) (`self.8`))))

(fn `UserConstructionScript`
  (`parent.UserConstructionScript`))