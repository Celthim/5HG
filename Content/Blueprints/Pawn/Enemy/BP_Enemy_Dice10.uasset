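; BP_Enemy_Dice10 is an enemy pawn Blueprint, named as a ten-sided die variant, with ten arrow references.
; Its InitArrow event appends the ten arrows to the Arrows array in a hand-set order that differs from their numbering.
; It adds no other logic: BeginPlay is a disabled stub and the construction script only calls the parent.
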(event `self.InitArrow`
  (`KismetArrayLibrary.Array_Append` (`self.Arrows`) (`|MakeArray` (`self.Arrow4`) (`self.Arrow8`) (`self.Arrow7`) (`self.Arrow6`) (`self.Arrow5`) (`self.Arrow9`) (`self.Arrow3`) (`self.Arrow2`) (`self.Arrow1`) (`self.Arrow`))))

(fn `UserConstructionScript`
  (`parent.UserConstructionScript`))