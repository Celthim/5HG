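; Ambient sound emitter that plays random one-shot sounds inside a box volume.
; From BeginPlay it picks a random entry from a sound array and plays it with attenuation at a random point in the box, centered on the root component.
; It then waits a random few seconds and calls itself again, looping indefinitely.
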(event `self.ReceiveBeginPlay`
  (`self.Spawn Sound`))

(event `Spawn Sound`
  (bind _tabofsounds (`self.TabOfSounds`))
  (`GameplayStatics.SpawnSoundAtLocation` (`|GetArrayItem` _tabofsounds (`KismetMathLibrary.RandomIntegerInRange` 0 (`KismetArrayLibrary.Array_LastIndex` _tabofsounds))) (`KismetMathLibrary.RandomPointInBoundingBox` (`SceneComponent.K2_GetComponentLocation` (`self.DefaultSceneRoot`)) (`BoxComponent.BoxExtent` (`self.Box`))) (struct) 1.0 1.0 0.0 "/Game/Sounds/NewSoundAttenuation.NewSoundAttenuation" null)
  (`KismetSystemLibrary.Delay` (`KismetMathLibrary.RandomFloatInRange` 4.0 8.0))
  (`self.Spawn Sound`))

(fn `UserConstructionScript`)